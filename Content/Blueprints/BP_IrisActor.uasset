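; BP_IrisActor is an actor with four prop components, each spun by its own rotating movement component.
; On BeginPlay it stores the four rotating movement components in an array and calls a setup function.
; That function sets each movement component's updated component to its matching prop, so each rotates independently of the others.
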(event `self.ReceiveBeginPlay`
  (set `self.RotatingComponents` (`|MakeArray` (`self.Prop0_Rotating`) (`self.Prop1_Rotating`) (`self.Prop2_Rotating`) (`self.Prop3_Rotating`)))
  (`self.SetupPropRotationMovement`))

(fn `SetupPropRotationMovement`
  (`MovementComponent.SetUpdatedComponent` (`self.Prop1_Rotating`) (`self.Prop1`))
  (`MovementComponent.SetUpdatedComponent` (`self.Prop3_Rotating`) (`self.Prop3`))
  (`MovementComponent.SetUpdatedComponent` (`self.Prop0_Rotating`) (`self.Prop0`))
  (`MovementComponent.SetUpdatedComponent` (`self.Prop2_Rotating`) (`self.Prop2`))
  (return))

(fn `UserConstructionScript`)