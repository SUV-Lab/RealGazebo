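; BP_RoverActor is a ground vehicle rover with four spinning wheels.
; On BeginPlay it fills RotatingComponents with four rotation movement components and binds each to its own wheel through SetUpdatedComponent.
; It then registers Wheel1 and Wheel2 as ControllableComponents; the logic that uses both arrays is not in this graph.
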(event `self.ReceiveBeginPlay`
  (set `self.RotatingComponents` (`|MakeArray` (`self.Rotation0`) (`self.Rotation1`) (`self.Rotation2`) (`self.Rotation3`)))
  (`self.SetupPropRotationMovement`)
  (set `self.ControllableComponents` (`|MakeArray` (`self.wheel1`) (`self.wheel2`))))

(fn `SetupPropRotationMovement`
  (`MovementComponent.SetUpdatedComponent` (`self.Rotation0`) (`self.wheel0`))
  (`MovementComponent.SetUpdatedComponent` (`self.Rotation1`) (`self.wheel1`))
  (`MovementComponent.SetUpdatedComponent` (`self.Rotation2`) (`self.wheel2`))
  (`MovementComponent.SetUpdatedComponent` (`self.Rotation3`) (`self.wheel3`))
  (return))

(fn `UserConstructionScript`)