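; BP_LC62Pawn is the LC62 UAV pawn in the RealGazeboBridge vehicle set, with six rotors, two pushers and five control surfaces.
; On BeginPlay it gathers eight rotation components into RotatingComponents and binds each to its rotor or pusher through SetUpdatedComponent.
; It also registers the ailerons, elevators and rudder in ControllableComponents.
; The Blueprint only wires up these parts, with no logic here that drives them.
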(event `self.ReceiveBeginPlay`
  (set `self.RotatingComponents` (`|MakeArray` (`self.Rotation0`) (`self.Rotation1`) (`self.Rotation2`) (`self.Rotation3`) (`self.Rotation4`) (`self.Rotation5`) (`self.Rotation6`) (`self.Rotation7`)))
  (`self.SetupPropRotationMovement`)
  (set `self.ControllableComponents` (`|MakeArray` (`self.Aileron_L`) (`self.Aileron_R`) (`self.Elevator_L`) (`self.Elevator_R`) (`self.Rudder`) :!type "SceneComponent Object Reference")))

(fn `SetupPropRotationMovement`
  (`MovementComponent.SetUpdatedComponent` (`self.Rotation0`) (`self.rotor_0`))
  (`MovementComponent.SetUpdatedComponent` (`self.Rotation1`) (`self.rotor_1`))
  (`MovementComponent.SetUpdatedComponent` (`self.Rotation2`) (`self.rotor_2`))
  (`MovementComponent.SetUpdatedComponent` (`self.Rotation3`) (`self.rotor_3`))
  (`MovementComponent.SetUpdatedComponent` (`self.Rotation4`) (`self.rotor_4`))
  (`MovementComponent.SetUpdatedComponent` (`self.Rotation5`) (`self.rotor_5`))
  (`MovementComponent.SetUpdatedComponent` (`self.Rotation6`) (`self.Pusher_L`))
  (`MovementComponent.SetUpdatedComponent` (`self.Rotation7`) (`self.Pusher_R`))
  (return))

(fn `UserConstructionScript`)