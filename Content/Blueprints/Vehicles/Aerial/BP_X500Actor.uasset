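; BP_X500Actor is an aerial vehicle actor, apparently an X500 quadcopter, that sets up rotation for its four propellers.
; On BeginPlay it gathers four rotation components into the RotatingComponents array, then calls SetupPropRotationMovement.
; That function sets each rotation component's updated component to its matching prop, so each propeller has its own rotation driver.
; The construction script is empty.
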(event `self.ReceiveBeginPlay`
  (set `self.RotatingComponents` (`|MakeArray` (`self.Rotation0`) (`self.Rotation1`) (`self.Rotation2`) (`self.Rotation3`)))
  (`self.SetupPropRotationMovement`))

(fn `SetupPropRotationMovement`
  (`MovementComponent.SetUpdatedComponent` (`self.Rotation0`) (`self.Prop0`))
  (`MovementComponent.SetUpdatedComponent` (`self.Rotation1`) (`self.Prop1`))
  (`MovementComponent.SetUpdatedComponent` (`self.Rotation2`) (`self.Prop2`))
  (`MovementComponent.SetUpdatedComponent` (`self.Rotation3`) (`self.Prop3`))
  (return))

(fn `UserConstructionScript`)