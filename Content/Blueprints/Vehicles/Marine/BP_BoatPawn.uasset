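; Boat pawn Blueprint that wires up rotation movement for its two propellers.
; On BeginPlay it stores both rotation components in the RotatingComponents array, then calls SetupPropRotationMovement.
; That function uses SetUpdatedComponent to point each rotation component at its own prop, so each propeller turns independently of the hull.
; The construction script is empty, and no rotation rates or driving logic are set in these graphs.
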(event `self.ReceiveBeginPlay`
  (set `self.RotatingComponents` (`|MakeArray` (`self.Rotation0`) (`self.Rotation1`)))
  (`self.SetupPropRotationMovement`))

(fn `SetupPropRotationMovement`
  (`MovementComponent.SetUpdatedComponent` (`self.Rotation0`) (`self.Prop0`))
  (`MovementComponent.SetUpdatedComponent` (`self.Rotation1`) (`self.Prop1`))
  (return))

(fn `UserConstructionScript`)