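; BP_RoverActor is a rover actor with four wheels, each paired with its own rotating movement component.
; At BeginPlay it gathers the four rotating components into the RotatingComponents array, then calls SetupPropRotationMovement.
; That function sets each component's updated component to its matching wheel, so each wheel rotates independently of the actor root.
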(event `self.ReceiveBeginPlay`
  (set `self.RotatingComponents` (`|MakeArray` (`self.Wheel0_Rotating`) (`self.Wheel1_Rotating`) (`self.Wheel2_Rotating`) (`self.Wheel3_Rotating`)))
  (`self.SetupPropRotationMovement`))

(fn `SetupPropRotationMovement`
  (`MovementComponent.SetUpdatedComponent` (`self.Wheel1_Rotating`) (`self.wheel1`))
  (`MovementComponent.SetUpdatedComponent` (`self.Wheel3_Rotating`) (`self.wheel3`))
  (`MovementComponent.SetUpdatedComponent` (`self.Wheel0_Rotating`) (`self.wheel0`))
  (`MovementComponent.SetUpdatedComponent` (`self.Wheel2_Rotating`) (`self.wheel2`))
  (return))

(fn `UserConstructionScript`)