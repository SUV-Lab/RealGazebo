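; BP_BoatActor is a boat actor with two rotating propellers, Left and Right.
; On BeginPlay it stores the Motor0Rotating and Motor1Rotating movement components in a RotatingComponents array, then runs SetupPropRotationMovement.
; That function sets Left and Right as the updated components of the two motors, so each rotates its own prop rather than the whole actor.
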(event `self.ReceiveBeginPlay`
  (set `self.RotatingComponents` (`|MakeArray` (`self.Motor0_Rotating`) (`self.Motor1_Rotating`)))
  (`self.SetupPropRotationMovement`))

(fn `SetupPropRotationMovement`
  (`MovementComponent.SetUpdatedComponent` (`self.Motor0_Rotating`) (`self.Left`))
  (`MovementComponent.SetUpdatedComponent` (`self.Motor1_Rotating`) (`self.Right`))
  (return))

(fn `UserConstructionScript`)